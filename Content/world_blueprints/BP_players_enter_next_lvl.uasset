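; Level exit trigger actor that counts players standing in its box, intended to open the next level once two are present.
; BeginPlay caches the GI_Var_store game instance, whose PlayersMovingLVL counter rises on box begin overlap and falls on end overlap.
; Overlaps are not filtered by actor type, and reaching two only prints a debug message; no level is actually loaded.
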(event `self.ReceiveBeginPlay`
  (bind _asgi_var_store (cast `/Game/Globle/GI_Var_store` (`GameplayStatics.GetGameInstance`)))
  (set `self.As GI Var Store` _asgi_var_store))

(event `self.Box.OnComponentBeginOverlap`
  (params (OverlappedComponent :type "PrimitiveComponent Object Reference") (OtherActor :type "Actor Object Reference") (OtherComp :type "PrimitiveComponent Object Reference") (OtherBodyIndex :type Integer) (bFromSweep :type Boolean) (SweepResult :type "HitResult Structure (by ref)"))
  (bind _as_gi_var_store (`self.As GI Var Store`))
  (bind _output_get (set `/Game/Globle/GI_Var_store.players moving LVL` (+ (`/Game/Globle/GI_Var_store.players moving LVL` _as_gi_var_store) 1) _as_gi_var_store))
  (`KismetSystemLibrary.PrintString` (`KismetStringLibrary.Conv_IntToString` _output_get))
  (if (== (`/Game/Globle/GI_Var_store.players moving LVL` (`self.As GI Var Store`)) 2)
    (`KismetSystemLibrary.PrintString` "open new lv")))

(event `self.Box.OnComponentEndOverlap`
  (params (OverlappedComponent :type "PrimitiveComponent Object Reference") (OtherActor :type "Actor Object Reference") (OtherComp :type "PrimitiveComponent Object Reference") (OtherBodyIndex :type Integer))
  (bind _as_gi_var_store (`self.As GI Var Store`))
  (set `/Game/Globle/GI_Var_store.players moving LVL` (- (`/Game/Globle/GI_Var_store.players moving LVL` _as_gi_var_store) 1) _as_gi_var_store)
  (`KismetSystemLibrary.PrintString` "player left  trigger"))

(fn `UserConstructionScript`)